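; BP_SingleMainGameMode is a game mode that chooses the player start based on whether the dungeon is ready.
; FindPlayerStart returns the first PlayerStart in the level once IsDungeonReady is set, otherwise falling back to the parent implementation.
; OnSpawnRoomsLoaded sets that flag, but the code binding it to the Dungeon's level streaming initial-chunks-loaded event is disconnected and never runs.
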(event Custom|OnSpawnRoomsLoaded
  (params (Dungeon :type Dungeon%20Object%20Reference))
  ;[1 1 1] Setup Level Streaming
  (Variables|Default|SetbIsDungeonReady true))

(event EventBeginPlay)

(event EventTick
  (params (DeltaSeconds :type Float%20%28single-precision%29)))

(fn ConstructionScript)

(fn FindPlayerStart
  (params (Player :type Controller%20Object%20Reference) (IncomingName :type String))
  (if (Variables|Default|GetbIsDungeonReady)
    (bind _outactors (Actor|GetAllActorsOfClass "/Script/Engine.PlayerStart"))
    (if (> (Utilities|Array|Length _outactors) 0)
      (return (Utilities|Array|Get(acopy) _outactors))
      (else
        _)))
  (bind _returnvalue (|CallParentFunction Player IncomingName))
  (return _returnvalue))