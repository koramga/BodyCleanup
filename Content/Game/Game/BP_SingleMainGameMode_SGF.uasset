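; Single-player game mode that generates a randomized streamed dungeon and holds match start until it is ready.
; On BeginPlay it finds the Dungeon actor, binds to its level streaming model's initial-chunks-loaded callback, randomizes the seed and builds.
; That callback sets DungeonReady, which gates ReadyToStartMatch.
; FindPlayerStart then picks the first PlayerStart in the world, falling back to parent logic if unready or none exists.
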(event Custom|OnSpawnRoomsLoaded
  (params (Dungeon :type Dungeon%20Object%20Reference))
  ;[1 1 1] Setup Level Streaming
  (Variables|Default|SetDungeonReady true))

(event EventBeginPlay
  (Utilities|FlowControl|Sequence
    (:then_0
      ;[1 1 1] Setup Level Streaming
      (bind _returnvalue (Actor|GetActorOfClass "/Script/DungeonArchitectRuntime.Dungeon"))
      (bind _output_get (Variables|Default|SetDungeon _returnvalue))
      (Utilities|IsValid _output_get
        (:Is%20Valid
          (EventDispatchers|AssignOnInitialChunksLoaded (Variables|/Script/DungeonArchitectRuntime.Dungeon|GetLevelStreamingModel _output_get) (delegate Custom|OnSpawnRoomsLoaded)))))
    (:then_1
      ;[1 1 1] Randomize dungeon
      (Variables|/Script/DungeonArchitectRuntime.DungeonConfig|SetSeed (Variables|/Script/DungeonArchitectRuntime.Dungeon|GetConfig (Variables|Default|GetDungeon)) (Math|Random|RandomInteger 10000000)))
    (:then_2
      ;[1 1 1] Build Dungeon
      (Class|Dungeon|BuildDungeon (Variables|Default|GetDungeon)))))

(event EventTick
  (params (DeltaSeconds :type Float%20%28single-precision%29)))

(fn ConstructionScript)

(fn ReadytoStartMatch
  (return (Variables|Default|GetDungeonReady)))

(fn FindPlayerStart
  (params (Player :type Controller%20Object%20Reference) (IncomingName :type String))
  (if (Variables|Default|GetDungeonReady)
    (bind _outactors (Actor|GetAllActorsOfClass "/Script/Engine.PlayerStart"))
    (if (> (Utilities|Array|Length _outactors) 0)
      (return (Utilities|Array|Get(acopy) _outactors))
      (else
        _)))
  (bind _returnvalue (|CallParentFunction Player IncomingName))
  (return _returnvalue))